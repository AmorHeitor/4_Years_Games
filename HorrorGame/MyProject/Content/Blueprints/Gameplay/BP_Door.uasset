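; BP_Door is a double door that swings open and closed through its Open and Close events.
; Separate timelines rotate the left and right leaves, lerping from their current rotation toward fixed yaw targets along the shortest path.
; Open acts as a toggle via IsOpen, calling Close when the flag is false.
; IsOpen reads inverted: it becomes false after opening finishes and true after closing finishes.
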(event `Open`
  (bind _doorright (`self.DoorRight`))
  (bind _doorleft (`self.DoorLeft`))
  ;[1 0.8672 0] Opens the door
  (if (`self.bIsOpen`)
    (bind (_direction _alpha) (`Timeline|OpenDoor` :!via `PlayFromStart`)
      (:`Update`
        (`SceneComponent.K2_SetRelativeRotation` _doorright (`KismetMathLibrary.RLerp` (`SceneComponent.RelativeRotation` _doorright) (struct :`Yaw` -90.0) _alpha true) false false)
        (`SceneComponent.K2_SetRelativeRotation` _doorleft (`KismetMathLibrary.RLerp` (`SceneComponent.RelativeRotation` _doorleft) (struct :`Yaw` -270.0) _alpha true) false false))
      (:`Finished`
        (set `self.bIsOpen` false)))
    (else
      (`self.Close`))))

(event `Close`
  (bind _doorright (`self.DoorRight`))
  (bind _doorleft (`self.DoorLeft`))
  ;[1 0 0.1641] Closes the door
  (bind (_direction _alpha) (`Timeline|CloseDoor` :!via `PlayFromStart`)
    (:`Update`
      (`SceneComponent.K2_SetRelativeRotation` _doorright (`KismetMathLibrary.RLerp` (`SceneComponent.RelativeRotation` _doorright) (struct :`Yaw` -180.0) _alpha true) false false)
      (`SceneComponent.K2_SetRelativeRotation` _doorleft (`KismetMathLibrary.RLerp` (`SceneComponent.RelativeRotation` _doorleft) (struct :`Yaw` -180.0) _alpha true) false false))
    (:`Finished`
      (set `self.bIsOpen` true))))

(fn `UserConstructionScript`)