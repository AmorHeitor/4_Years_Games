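; Player blueprint that handles overlap-based interaction and a right-mouse projectile throw.
; Interact messages every actor overlapping the Interact component.
; Holding right mouse starts a looping timer that draws a predicted projectile path and stores its hit location.
; Release spawns BP_Projectile and timeline-lerps it to that point from the raw camera forward vector, not the player's position; the impulse launch and timer clearing are unconnected.
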(event `InputAction|Interact`
  (params (Key :type "Key Structure"))
  ;[1 0.1172 0] Interaction
  (:`Pressed`
    (for _array_element (`PrimitiveComponent.GetOverlappingActors` (`self.Interact`) null)
      (message `/Game/Blueprints/Library/BP_Interaction.OnInteract` _array_element))))

(event `Key|RightMouseButton`
  (params (Key :type "Key Structure"))
  (:`Pressed`
    (bind _returnvalue (`KismetSystemLibrary.K2_SetTimer` null "PredictPath" 0.5 true)))
  (:`Released`
    (`self.Flying`)))

(event `PredictPath`
  (bind _returnvalue (`SceneComponent.GetForwardVector` (`self.CameraComp`)))
  (bind _outhit (`GameplayStatics.Blueprint_PredictProjectilePath_ByTraceChannel` (+ (+ (`self.K2_GetActorLocation`) (50.0 50.0 0.0)) (* _returnvalue 75)) (* _returnvalue 2500) true 15.0 "ECC_WorldDynamic" false (`|MakeArray` self :!type "Actor Object Reference") "ForDuration" 0.5))
  (set `self.ProjectileLocation` (`.Location` (`GameplayStatics.BreakHitResult` _outhit))))

(event `Flying`
  (bind _returnvalue (`|SpawnActorFromClass` "/Game/Blueprints/Gameplay/BP_Projectile.BP_Projectile_C" (`KismetMathLibrary.MakeTransform` (`SceneComponent.GetForwardVector` (`self.CameraComp`)) (struct) (0.2 0.2 0.2)) "Undefined" "OverrideRootScale" null null))
  (bind (_direction _alpha) (`Timeline|ProjectileFly`)
    (:`Update`
      (`self.K2_SetActorLocation` _returnvalue (`KismetMathLibrary.VLerp` (`SceneComponent.GetForwardVector` (`self.CameraComp`)) (`self.ProjectileLocation`) _alpha) false false))))

(fn `UserConstructionScript`)